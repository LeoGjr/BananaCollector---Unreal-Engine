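; BP_Player is the player pawn in BananaCollector, moved along its forward and right vectors by axis inputs.
; The MoveForward and MoveRight events add movement input scaled by axis value and MaxSpeed.
; Tick consumes the accumulated input vector and applies it as a delta-time-scaled local offset with sweep, so movement is done by hand in the graph.
; The world-space input vector is applied as a local offset, so directions match only while the actor is unrotated.
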(event `self.ReceiveTick`
  (params (DeltaSeconds :type "Float (single-precision)"))
  ;[1 1 1] Altera a localização do player com base nos inputs
  (bind _returnvalue (`self.ConsumeMovementInputVector`))
  (`self.K2_AddActorLocalOffset` (* DeltaSeconds _returnvalue) true))

(event `InputAxis|MoveRight`
  (params (AxisValue :type "Float (single-precision)"))
  ;[1 1 1] Cria movimentos de entrada com base nos inputs
  (`self.AddMovementInput` (`self.GetActorRightVector`) (* AxisValue (`self.MaxSpeed`))))

(event `InputAxis|MoveForward`
  (params (AxisValue :type "Float (single-precision)"))
  ;[1 1 1] Adiciona movimentos de entrada ao objeto
  (`self.AddMovementInput` (`self.GetActorForwardVector`) (* (`self.MaxSpeed`) AxisValue)))

(fn `UserConstructionScript`)